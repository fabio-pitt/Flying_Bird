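; Menu HUD Blueprint that puts the main menu widget on screen at BeginPlay.
; CreateMenuScreen creates WBP_Menu for player 0, adds it to the viewport and sets UI-only input focused on it.
; A desktop splash path, skipped on Android and handing off to the menu when its animation ends, is present but disconnected, so it never runs.
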(event `self.ReceiveBeginPlay`
  (`self.CreateMenuScreen`))

(event `RemoveSplash`
  (`Widget.RemoveFromParent` (`self.SplashScreen`))
  (`self.CreateMenuScreen`))

(fn `CreateMenuScreen`
  (bind _returnvalue (`|CreateWidget` "/Game/Widgets/WBP_Menu.WBP_Menu_C" (`GameplayStatics.GetPlayerController` 0)))
  (bind _output_get (set `self.Menu` _returnvalue))
  (`/Engine/EditorBlueprintResources/StandardMacros.IsValid` _output_get
    (:`Is Valid`
      (`UserWidget.AddToViewport` (`self.Menu`) 0)
      (`WidgetBlueprintLibrary.SetInputMode_UIOnlyEx` (`GameplayStatics.GetPlayerController` 0) (`self.Menu`) "LockOnCapture")
      (return))))

(fn `CreateSplashScreen`
  (bind _returnvalue (`GameplayStatics.GetPlayerController` 0))
  (bind _returnvalue_2 (`|CreateWidget` "/Game/Widgets/WBP_SplashScreen_Desktop.WBP_SplashScreen_Desktop_C" _returnvalue))
  (bind _output_get (set `self.SplashScreen` _returnvalue_2))
  (`/Engine/EditorBlueprintResources/StandardMacros.IsValid` _output_get
    (:`Is Valid`
      (`UserWidget.AddToViewport` _output_get 0)
      (`WidgetBlueprintLibrary.SetInputMode_UIOnlyEx` _returnvalue _output_get "LockOnCapture"))))

(fn `UserConstructionScript`)